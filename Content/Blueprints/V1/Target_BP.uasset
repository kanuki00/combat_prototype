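; Targetable actor that displays lock-on markers and reacts to damage with knockback.
; Creates confirmed and suggested target widgets at the mesh's TARGET socket, then each tick shows one or neither based on the player character's Target and SuggestedTarget.
; Damage plays a mesh scale timeline and pushes Collision away from the instigator's pawn with an impulse scaled by damage.
; A Tick-driven cooldown timer blocks repeated hit reactions.
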(event Custom|DamageEffect
  (bind _newscale (Timeline|Scale PlayFromStart)
    (:Update
      (Transformation|SetRelativeScale3D (Variables|Default|GetMesh) (Math|Vector|MakeVector _newscale _newscale _newscale)))))

(event EventTick
  (params (DeltaSeconds :type Float%20%28single-precision%29))
  (Utilities|FlowControl|Sequence
    (:then_0
      (if (not (Variables|Actor|GetbCanBeDamaged))
        (if (>= (Variables|Default|GetDamageCooldownTimer) (Variables|Default|GetDamageCooldownLength))
          (Variables|Actor|SetbCanBeDamaged true)
          (Variables|Default|SetDamageCooldownTimer 0.0)
          (else
            (Variables|Default|SetDamageCooldownTimer (+ (Utilities|Time|GetWorldDeltaSeconds) (Variables|Default|GetDamageCooldownTimer)))))))
    (:then_1
      (|TargetingWidgetPlacing))
    (:then_2
      (bind _asplayer_character (Utilities|Casting|CastToPlayerCharacter (Game|GetPlayerCharacter 0)))
      (Development|PrintString (Utilities|String|ToString(Boolean) (== self (Variables|/Script/UE5_CombatProto.PlayerCharacter|GetSuggestedTarget _asplayer_character))) false false "(R=0.000000,G=0.660000,B=1.000000,A=1.000000)" (Utilities|Time|GetWorldDeltaSeconds)))))

(event EventBeginPlay
  (bind _returnvalue (UserInterface|CreateWidget "/Game/Blueprints/WidgetBlueprints/FloatingWidget_WBP.FloatingWidget_WBP_C" 0 "/Game/Assets/Textures/Target.Target" "TARGET" (Variables|Default|GetMesh)))
  (Variables|Default|SetTarget _returnvalue)
  (bind _returnvalue_2 (UserInterface|CreateWidget "/Game/Blueprints/WidgetBlueprints/FloatingWidget_WBP.FloatingWidget_WBP_C" 0 "/Game/Assets/Textures/TargetSuggest.TargetSuggest" "TARGET" (Variables|Default|GetMesh)))
  (Variables|Default|SetSuggestedTarget _returnvalue_2))

(event Game|Damage|EventAnyDamage
  (params (Damage :type Float%20%28single-precision%29) (DamageType :type Damage%20Type%20Object%20Reference) (InstigatedBy :type Controller%20Object%20Reference) (DamageCauser :type Actor%20Object%20Reference))
  (if (Variables|Actor|GetbCanBeDamaged)
    (Variables|Actor|SetbCanBeDamaged false)
    (CallFunction|DamageEffect)
    (Physics|AddImpulse (Variables|Default|GetCollision) (* (Math|Vector|Normalize (- (Transformation|GetActorLocation) (Transformation|GetActorLocation (Pawn|GetControlledPawn InstigatedBy)))) (* 6e+04 Damage)) "None" false)))

(fn ConstructionScript)