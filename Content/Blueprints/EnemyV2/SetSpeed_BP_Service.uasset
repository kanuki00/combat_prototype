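; Behavior tree service that sets the walk speed of an AI-controlled BaseCharacterV2 pawn.
; On AI activation it casts the controlled pawn, then picks either the character's default max walk speed or a custom new speed based on a toggle.
; It writes the chosen value to the character movement's max walk speed once per activation, with no tick or deactivation logic.
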(event EventReceiveActivationAI
  (params (OwnerController :type AI%20Controller%20Object%20Reference) (ControlledPawn :type Pawn%20Object%20Reference))
  (bind _asbase_character_v2 (Utilities|Casting|CastToBaseCharacterV2 ControlledPawn))
  (Utilities|FlowControl|Sequence
    (:then_0
      (if (Variables|Default|GetUseDefault)
        (Variables|Default|SetSpeed (Variables|/Script/UE5_CombatProto.BaseCharacterV2|GetDefaultMaxWalkSpeed _asbase_character_v2))
        (else
          (Variables|Default|SetSpeed (Variables|Default|GetNewWalkSpeed)))))
    (:then_1
      (Variables|/Script/Engine.CharacterMovementComponent|SetMaxWalkSpeed (Variables|/Script/Engine.Character|GetCharacterMovement _asbase_character_v2) (Variables|Default|GetSpeed)))))