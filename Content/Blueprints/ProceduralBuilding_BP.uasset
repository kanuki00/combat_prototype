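; Procedural building actor that assembles a hollow rectangular shell from modular meshes, sized by Width, Depth and Height.
; The construction script loops over the grid and keeps only perimeter cells on each level, adding instances to the Corner component at the four corners and to Face along the edges.
; Collapsed graphs handle the perimeter and corner tests, compute grid-spaced locations and derive each piece's yaw from its side.
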(event EventBeginPlay)

(event Collision|EventActorBeginOverlap
  (params (OtherActor :type Actor%20Object%20Reference)))

(event EventTick
  (params (DeltaSeconds :type Float%20%28single-precision%29)))

(fn ConstructionScript
  (for _index (range 0 (- (Variables|Default|GetHeight) 1))
    (for _index_2 (range 0 (- (Variables|Default|GetDepth) 1))
      (for _index_3 (range 0 (- (Variables|Default|GetWidth) 1))
        (if (|CollapseGraph_3 _index_2 _index_3) ; Wether to add instance
          (if (|CollapseGraph_0 _index_2 _index_3)
            (Components|InstancedStaticMesh|AddInstance (Variables|Default|GetCorner) (Math|Transform|MakeTransform (|CollapseGraph_2 _index _index_2 _index_3) (Math|Rotator|MakeRotator 0.0 0.0 (|CollapseGraph_1 _index_2 _index_3)) "1.000000,1.000000,1.000000") false)
            (else
              (Components|InstancedStaticMesh|AddInstance (Variables|Default|GetFace) (Math|Transform|MakeTransform (|CollapseGraph_2 _index _index_2 _index_3) (Math|Rotator|MakeRotator 0.0 0.0 (|CollapseGraph_1 _index_2 _index_3)) "1.000000,1.000000,1.000000") false))))))))