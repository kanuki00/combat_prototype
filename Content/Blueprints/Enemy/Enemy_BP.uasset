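; Enemy character that equips a sword and shows screen markers when the player targets it.
; On BeginPlay it attaches a spawned Sword to the right-hand socket and creates two FloatingWidget_WBP widgets tied to the mesh's TARGET socket.
; Every Tick it compares itself to the PlayerCharacter's Target and SuggestedTarget, showing the matching marker or removing both, with Target taking priority.
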(event EventTick
  (params (DeltaSeconds :type Float%20%28single-precision%29))
  (|TargetingWidgetPlacing_2))

(event EventBeginPlay
  (bind _returnvalue (Game|SpawnActorfromClass "/Game/Blueprints/Sword.Sword_C" (Math|Transform|MakeTransform "0, 0, 0" "0, 0, 0" "1.000000,1.000000,1.000000") "Undefined" 0 0))
  (Transformation|AttachComponentToComponent _returnvalue (Variables|Character|GetMesh) "equip_hand_right" "SnapToTarget" "SnapToTarget" "SnapToTarget" true)
  (bind _returnvalue_2 (UserInterface|CreateWidget "/Game/Blueprints/WidgetBlueprints/FloatingWidget_WBP.FloatingWidget_WBP_C" 0 "/Game/Assets/Textures/Target.Target" "TARGET" (Variables|Character|GetMesh)))
  (Variables|Default|SetTargetWBP _returnvalue_2)
  (bind _returnvalue_3 (UserInterface|CreateWidget "/Game/Blueprints/WidgetBlueprints/FloatingWidget_WBP.FloatingWidget_WBP_C" 0 "/Game/Assets/Textures/TargetSuggest.TargetSuggest" "TARGET" (Variables|Character|GetMesh)))
  (Variables|Default|SetSuggestedTargetWBP _returnvalue_3))

(fn ConstructionScript)