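; Enemy AI behavior tree task that picks a random wander point around the controlled pawn and writes it to the Location blackboard key.
; It samples a reachable navmesh point within Radius of the pawn.
; Points closer than MinimumRadius are replaced by one at that distance in the opposite direction, without a reachability recheck.
; The task always finishes successfully, and its debug distance print has both screen and log output disabled.
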(event EventReceiveExecuteAI
  (params (OwnerController :type AI%20Controller%20Object%20Reference) (ControlledPawn :type Pawn%20Object%20Reference))
  (bind _returnvalue (Transformation|GetActorLocation ControlledPawn))
  (bind _returnvalue_2 (Transformation|GetActorLocation ControlledPawn))
  (bind _returnvalue_3 (Transformation|GetActorLocation ControlledPawn))
  (bind _radius (Variables|Default|GetRadius))
  (bind _minimumradius (Variables|Default|GetMinimumRadius))
  (bind _randomlocation (AI|Navigation|GetRandomReachablePointinRadius _returnvalue_3 _radius 0 0))
  (bind _returnvalue_4 (Math|Vector|Distance(Vector) _randomlocation _returnvalue))
  (bind _returnvalue_5 (- _returnvalue _randomlocation))
  (bind _returnvalue_6 (Math|Vector|Normalize _returnvalue_5))
  (bind _returnvalue_7 (< _returnvalue_4 _minimumradius))
  (bind _returnvalue_8 (* _returnvalue_6 _minimumradius))
  (bind _returnvalue_9 (+ _returnvalue_8 _returnvalue_2))
  (bind _returnvalue_10 (Math|Vector|SelectVector _returnvalue_9 _randomlocation _returnvalue_7))
  (Development|PrintString (Utilities|String|ToString(Float) (Math|Vector|VectorLength (- (Transformation|GetActorLocation ControlledPawn) _returnvalue_10))) false false "(R=0.024933,G=1.000000,B=0.000000,A=1.000000)")
  (AI|BehaviorTree|SetBlackboardValueasVector (Variables|Default|GetLocation) _returnvalue_10)
  (AI|BehaviorTree|FinishExecute true))