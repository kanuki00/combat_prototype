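; Main player character Blueprint that sets up the sword, HUD, camera zoom and restart on death.
; BeginPlay spawns a Sword, attaches it to the mesh's right-hand equip socket and adds the HUD widget to the viewport.
; Mouse wheel input adjusts a target boom length, seeded from the camera boom at construction, and interpolates the arm toward it.
; Tick polls IsDead and, once true, reloads CityLevel after a delay.
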(event EventBeginPlay
  (bind _returnvalue (Game|SpawnActorfromClass "/Game/Blueprints/Weapons/Sword.Sword_C" (Math|Transform|MakeTransform "0, 0, 0" "0, 0, 0" "1.000000,1.000000,1.000000") "Undefined" 0 0))
  (Transformation|AttachComponentToComponent _returnvalue (Variables|Character|GetMesh) "equip_hand_right" "SnapToTarget" "SnapToTarget" "SnapToTarget" true)
  (bind _returnvalue_2 (UserInterface|CreateWidget "/Game/Blueprints/WidgetBlueprints/HUD_WBP.HUD_WBP_C"))
  (UserInterface|Viewport|AddtoViewport _returnvalue_2 0))

(event EventTick
  (params (DeltaSeconds :type Float%20%28single-precision%29))
  ;[1 1 1] Quick and dirty game restarting
  (if (Variables|Default|GetIsDead)
    (Utilities|FlowControl|DoOnce false
      (:Completed
        (Utilities|FlowControl|Delay 5.0)
        (Game|OpenLevel(byName) "CityLevel")))))

(event Input|MouseEvents|MouseWheelAxis
  (params (AxisValue :type Float%20%28single-precision%29))
  (Variables|Default|SetNewBoomLength (+ (* AxisValue -2e+01) (Variables|Default|GetNewBoomLength)))
  (Variables|/Script/Engine.SpringArmComponent|SetTargetArmLength (Variables|Default|GetCameraBoom) (Math|Interpolation|FInterpTo (Variables|/Script/Engine.SpringArmComponent|GetTargetArmLength (Variables|Default|GetCameraBoom)) (Variables|Default|GetNewBoomLength) (Utilities|Time|GetWorldDeltaSeconds) 5.0)))

(fn ConstructionScript
  (Variables|Default|SetNewBoomLength (Variables|/Script/Engine.SpringArmComponent|GetTargetArmLength (Variables|Default|GetCameraBoom))))